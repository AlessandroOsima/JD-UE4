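; VR player Blueprint that lets the player aim and use powers and teleport with the right motion controller.
; BeginPlay initializes the PowerRaycaster's powers with a delayed start.
; Each Tick, a long ray from the Arrow component against a floor trace channel sets whether a power can be used.
; Right trigger fires the power when allowed, and right thumbstick press teleports to the last valid position.
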(event EventBeginPlay
  (Class|JDBlueprintFunctionLibrary|SetPowersStart (Variables|/Script/BaseBlank.PowerRayCasterComponent|GetPowers (Variables|Default|GetPowerRaycaster)) "Delayed"))

(event Collision|EventActorBeginOverlap
  (params (OtherActor :type Actor%20Object%20Reference)))

(event EventTick
  (params (DeltaSeconds :type Float%20%28single-precision%29))
  (bind _arrow (Variables|Default|GetArrow))
  (bind _returnvalue (Transformation|GetWorldLocation _arrow))
  ;[1 1 1] Raycast from controller to terrain and use power
  (bind _returnvalue_2 (Class|VrCamera|DoTargetRaycast _returnvalue (+ _returnvalue (* (Math|Vector|GetForwardVector (Variables|Default|GetArrow)) 1e+04)) "ECC_GameTraceChannel2"))
  (Variables|Default|SetCanUsePower _returnvalue_2))

(event Input|KeyboardEvents|MotionControllerRightThumbstick
  (params (Key :type Key%20Structure :default "AnyKey"))
  ;[1 1 1] Teleport
  (:Pressed
    (Class|VrCamera|TeleporttoLastValidPosition)))

(event Input|KeyboardEvents|MotionControllerRightTrigger
  (params (Key :type Key%20Structure :default "AnyKey"))
  ;[1 1 1] Use Power
  (:Pressed
    (if (Variables|Default|GetCanUsePower)
      (Class|PowerRayCasterComponent|UsePower (Variables|Default|GetPowerRaycaster)))))

(fn ConstructionScript)