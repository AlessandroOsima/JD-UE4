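; Player targeting indicator: a colored disc that hovers over, selects and attaches to actors with an active PowerInteractionsComponent.
; Box overlaps drive the hover state, while SwitchTargetState toggles selection, scaling to the target's sphere collider.
; State changes recolor the dynamic material and switch world collision between block and ignore.
; The target is released on hit, interaction start, component deactivation or, optionally, when Tick detects non-power objects overlapping the disc.
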(event Custom|EndOverlap
  (params (OtherActor :type Actor%20Object%20Reference) (OtherComp :type Primitive%20Component%20Object%20Reference) (OtherBodyIndex :type Integer))
  ;[1 1 1] End Overlap
  (bind _returnvalue (Class|IndicatorPawn|HasTarget))
  (if (not _returnvalue)
    (Class|IndicatorPawn|SetState "NoTarget")))

(event Custom|HitEvent
  (params (SelfActor :type Actor%20Object%20Reference) (OtherActor :type Actor%20Object%20Reference) (NormalImpulse :type Vector) (Hit :type Hit%20Result%20Structure%20%28by%20ref%29))
  ;[1 1 1] Hit
  (Class|IndicatorPawn|HasTarget)
  (if true
    (Class|IndicatorPawn|RemoveTarget)))

(event Custom|BeginOverlap
  (params (OtherActor :type Actor%20Object%20Reference) (OtherComp :type Primitive%20Component%20Object%20Reference) (OtherBodyIndex :type Integer) (bFromSweep :type Boolean) (SweepResult :type Hit%20Result%20Structure%20%28by%20ref%29))
  ;[1 1 1] Begin Overlap
  (bind _returnvalue (Class|IndicatorPawn|HasTarget))
  (if (not _returnvalue)
    (Class|IndicatorPawn|SetState "HoverOnTarget")))

(event EventSwitchTargetState
  ;[1 1 1] Switch Target State
  (bind _returnvalue (Class|IndicatorPawn|HasTarget))
  (if _returnvalue
    (Class|IndicatorPawn|UnsetTarget)
    (CallFunction|SetHoverStateonOverlap)
    (else
      ;[1 1 1] Select Target
      (bind _actorswithpowerinteractions (Class|JDBlueprintFunctionLibrary|GetActorswithPowerInteractionComponent (Collision|GetOverlappingActors (Variables|Default|GetBox) 0 :!class /Script/Engine.PrimitiveComponent)))
      (for _array_element _actorswithpowerinteractions
        (bind _returnvalue_2 (Class|JDBlueprintFunctionLibrary|GetPowerInteractionsComponent _array_element))
        (if (Components|Activation|IsActive _returnvalue_2)
          (Class|IndicatorPawn|ScaletoSphereCollider _array_element)
          (Class|IndicatorPawn|SetTarget _array_element))))))

(event EventTick
  (params (DeltaSeconds :type Float%20%28single-precision%29))
  ;[1 1 1] Check If target is still active
  (bind _returnvalue (Class|IndicatorPawn|HasTarget))
  (if _returnvalue
    (bind _returnvalue_2 (Class|IndicatorPawn|GetTarget))
    (if (> (Utilities|Array|Length (Actor|GetComponentsByClass _returnvalue_2 "/Script/BaseBlank.PowerInteractionsComponent")) 0)
      (if (Components|Activation|IsActive (Utilities|Array|Get(acopy) (Actor|GetComponentsByClass _returnvalue_2 "/Script/BaseBlank.PowerInteractionsComponent")))
        (if (Variables|Default|GetEnableDetachOnOverlap)
          ;[1 1 1] Check if disc is colliding with another actor
          (bind (_outactors _returnvalue_3) (Class|KismetSystemLibrary|ComponentOverlapActorsNEW (Variables|Default|GetObjectsCollision) (Transformation|GetActorTransform) (Utilities|Array|MakeArray "ObjectTypeQuery9") 0 (Variables|Default|GetActorsToIgnore)))
          (if _returnvalue_3
            (bind _array_element (Utilities|Array|ForEachLoopwithBreak _outactors :!label _label)
              (:LoopBody
                (bind _returnvalue_4 (Class|JDBlueprintFunctionLibrary|IsPowerEffect _array_element))
                (bind _returnvalue_5 (Class|JDBlueprintFunctionLibrary|IsPowerActor _array_element))
                (if (not (or _returnvalue_4 _returnvalue_5))
                  (Class|IndicatorPawn|RemoveTarget)
                  (goto _label Break))))))
        (else
          (Class|IndicatorPawn|RemoveTarget))))))

(event EventBeginPlay
  (bind _box (Variables|Default|GetBox))
  ;[1 1 1] Bind Event on Begin Play
  (Collision|BindEventtoOnComponentBeginOverlap _box (delegate Custom|BeginOverlap))
  (Collision|BindEventtoOnComponentEndOverlap _box (delegate Custom|EndOverlap))
  (EventDispatchers|BindEventtoOnActorHit (delegate Custom|HitEvent)))

(event EventOnIndicatorStateChanged
  (params (State :type EIndicatorTargetingState%20Enum :default "NoTarget"))
  (bind _collisionchannelresponse (Utilities|Struct|MakeCollisionChannelResponse "ECC_WorldStatic" "ECR_Ignore"))
  (bind _collisionchannelresponse_2 (Utilities|Struct|MakeCollisionChannelResponse "ECC_WorldDynamic" "ECR_Ignore"))
  (bind _collisionchannelresponse_3 (Utilities|Struct|MakeCollisionChannelResponse "ECC_WorldStatic" "ECR_Block"))
  (bind _collisionchannelresponse_4 (Utilities|Struct|MakeCollisionChannelResponse "ECC_WorldDynamic" "ECR_Block"))
  (bind _array (Utilities|Array|MakeArray _collisionchannelresponse _collisionchannelresponse_2))
  (bind _array_2 (Utilities|Array|MakeArray _collisionchannelresponse_3 _collisionchannelresponse_4))
  ;[1 1 1] Set Indicator Color
  (switch Utilities|FlowControl|Switch|SwitchonEIndicatorTargetingState State
    (:NoTarget
      (Rendering|Material|SetVectorParameterValue (Variables|Default|GetMaterialInstance) "Color" (Variables|Default|GetNoTargetSelectedColor) :!class /Script/Engine.MaterialInstanceDynamic)
      (Class|PrimitiveComponent|SetCollisionResponsestoChannels (Variables|Default|GetBox) _array_2)
      (Class|PrimitiveComponent|SetCollisionResponsestoChannels (Variables|Default|GetObjectsCollision) _array_2))
    (:HoverOnTarget
      (Rendering|Material|SetVectorParameterValue (Variables|Default|GetMaterialInstance) "Color" (Variables|Default|GetTargetSelectedColor) :!class /Script/Engine.MaterialInstanceDynamic))
    (:MoveToTarget
      (Class|PrimitiveComponent|SetCollisionResponsestoChannels (Variables|Default|GetBox) _array :!label _label)
      (Class|PrimitiveComponent|SetCollisionResponsestoChannels (Variables|Default|GetObjectsCollision) _array))
    (:OnTarget
      (Rendering|Material|SetVectorParameterValue (Variables|Default|GetMaterialInstance) "Color" (Variables|Default|GetTargetFollowColor) :!class /Script/Engine.MaterialInstanceDynamic)
      (goto _label))))

(event EventRemoveTarget
  ;[1 1 1] Remove Target Callback
  (bind _returnvalue (Class|IndicatorPawn|HasTarget))
  (if _returnvalue
    (Class|IndicatorPawn|UnsetTarget)
    (CallFunction|SetHoverStateonOverlap)))

(event EventOnTargetStartInteraction
  (params (Interaction :type Waypoint%20Interaction%20Component%20Object%20Reference))
  ;[1 1 1] Remove Indicator on interaction start
  (Class|IndicatorPawn|RemoveTarget))

(fn ConstructionScript
  (bind _returnvalue (Rendering|Material|CreateDynamicMaterialInstance (Variables|Default|GetDisc) 0 0 :!class /Script/Engine.PrimitiveComponent))
  (Variables|Default|SetMaterialInstance _returnvalue)
  (Utilities|Array|Add (Variables|Default|GetActorsToIgnore) self))

(fn SetHoverStateonOverlap
  ;[1 1 1] If overlap set state to hover
  (bind _returnvalue (Class|KismetSystemLibrary|ComponentOverlapActorsNEW (Variables|Default|GetBox) (Transformation|GetActorTransform) (Utilities|Array|MakeArray "ObjectTypeQuery3" "ObjectTypeQuery1" "ObjectTypeQuery2" "ObjectTypeQuery1")))
  (if _returnvalue
    (Class|IndicatorPawn|SetState "HoverOnTarget"))
  (return))