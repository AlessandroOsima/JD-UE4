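; BP_Player_Camera is the player camera Blueprint, which relays targeting input to an indicator pawn for targeting NPCs.
; Pressing SelectTarget casts the Indicator reference to IndicatorPawn and calls SwitchTargetState to target or untarget.
; The MoveForward and MoveSide axis events share one check that calls RemoveTarget on non-zero input, releasing the target when the indicator moves.
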(event Input|ActionEvents|InputActionSelectTarget
  (params (Key :type Key%20Structure :default "AnyKey"))
  ;[1 1 1] Target or untarget an npc
  (:Pressed
    (bind _asindicator_pawn (Utilities|Casting|CastToIndicatorPawn (Variables|Default|GetIndicator)))
    (Class|IndicatorPawn|SwitchTargetState _asindicator_pawn)))

(event Input|AxisEvents|InputAxisMoveForward
  (params (AxisValue :type Float%20%28single-precision%29))
  ;[1 1 1] Remove target If the indicator is moving away from it
  (bind _asindicator_pawn (Utilities|Casting|CastToIndicatorPawn (Variables|Default|GetIndicator)))
  (if (or (!= AxisValue 0.0) (!= (stale Input|AxisEvents|InputAxisMoveSide AxisValue) 0.0))
    (Class|IndicatorPawn|RemoveTarget _asindicator_pawn)))

(event Input|AxisEvents|InputAxisMoveSide
  (params (AxisValue :type Float%20%28single-precision%29))
  ;[1 1 1] Remove target If the indicator is moving away from it
  (bind _asindicator_pawn (Utilities|Casting|CastToIndicatorPawn (Variables|Default|GetIndicator)))
  (if (or (!= (stale Input|AxisEvents|InputAxisMoveForward AxisValue) 0.0) (!= AxisValue 0.0))
    (Class|IndicatorPawn|RemoveTarget _asindicator_pawn)))

(fn ConstructionScript)