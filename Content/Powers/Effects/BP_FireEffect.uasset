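; BP_FireEffect is a character effect that sets an NPC on fire and spreads by contact.
; StartUse pushes the fire behavior tree onto the NPCController, registers to the game mode, raises walk speed and applies a flame particle.
; A capsule hit handler gives a new fire effect to any BaseCharacter it strikes that has no effects.
; EndUse pops the tree, unregisters, restores speed and clears the particle, but leaves the hit binding.
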(event Custom|ActorHit
  (params (OtherActor :type Actor%20Object%20Reference) (OtherComp :type Primitive%20Component%20Object%20Reference) (NormalImpulse :type Vector) (Hit :type Hit%20Result%20Structure%20%28by%20ref%29))
  ;[1 1 1] Add effect on collision with another BaseCharacter
  (bind _asbase_character (Utilities|Casting|CastToBaseCharacter OtherActor))
  (bind _returnvalue (Class|JDBlueprintFunctionLibrary|CreateObject "BP_FireEffect_C" _asbase_character))
  (bind _asbase_effect (Utilities|Casting|CastToBaseEffect _returnvalue))
  (if (not (> (Utilities|Array|Length (Variables|/Script/BaseBlank.EffectComponent|GetEffects (Variables|/Script/BaseBlank.BaseCharacter|GetEffectComponent _asbase_character))) 0))
    (Class|EffectComponent|AddEffect (Variables|/Script/BaseBlank.BaseCharacter|GetEffectComponent _asbase_character) _asbase_effect)))

(event EventStartUse
  (params (Character :type Base%20Character%20Object%20Reference))
  (bind _returnvalue (Actor|GetComponentsByClass Character "/Script/Engine.CharacterMovementComponent"))
  (bind _item (Utilities|Array|Get(acopy) _returnvalue))
  ;[1 1 1] Add power bt to controller
  (Variables|Default|SetTime 0.0)
  (bind _asnpccontroller (Utilities|Casting|CastToNPCController (Pawn|GetController Character)))
  (Class|NPCController|PushNewBHTAsset _asnpccontroller "/Game/Powers/BHT_Power_Fire.BHT_Power_Fire")
  (Class|BaseEffect|RegistertoGameMode)
  ;[1 1 1] Set Character Speed
  (Variables|Default|SetCharacterSpeed (Class|MovementComponent|GetMaxSpeed _item))
  (Variables|/Script/Engine.CharacterMovementComponent|SetMaxWalkSpeed _item 8e+02)
  ;[1 1 1] Set Particle Effect
  (Effects|Components|ParticleSystem|SetTemplate (Utilities|Array|Get(acopy) (Actor|GetComponentsByClass Character "/Script/Engine.ParticleSystemComponent")) "/Game/Graph/Vectorfields/Particles/P_FlameShield.P_FlameShield")
  ;[1 1 1] Bind On Hit
  (Collision|BindEventtoOnComponentHit (Utilities|Array|Get(acopy) (Actor|GetComponentsByClass Character "/Script/Engine.CapsuleComponent")) (delegate Custom|ActorHit)))

(event EventEndUse
  (params (Character :type Base%20Character%20Object%20Reference))
  ;[1 1 1] Remove power bht
  (Variables|Default|SetTime 0.0)
  (bind _asnpccontroller (Utilities|Casting|CastToNPCController (Pawn|GetController Character)))
  (Class|NPCController|PopBHTAsset _asnpccontroller)
  (Class|BaseEffect|UnregisterfromGameMode)
  ;[1 1 1] Remove Particle Effect
  (Variables|/Script/Engine.CharacterMovementComponent|SetMaxWalkSpeed (Utilities|Array|Get(acopy) (Actor|GetComponentsByClass Character "/Script/Engine.CharacterMovementComponent")) (Variables|Default|GetCharacterSpeed))
  (Effects|Components|ParticleSystem|SetTemplate (Utilities|Array|Get(acopy) (Actor|GetComponentsByClass Character "/Script/Engine.ParticleSystemComponent")) 0))

(fn BeginOverlap
  (params (Other%20Actor :type Actor%20Object%20Reference) (Other%20Comp :type Primitive%20Component%20Object%20Reference) (Other%20Body%20Index :type Integer) (From%20Sweep :type Boolean) (Sweep%20Result :type Boolean)))