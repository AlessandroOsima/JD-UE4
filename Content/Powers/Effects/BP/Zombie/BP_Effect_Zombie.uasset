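; Zombie power effect that turns an NPC into a zombie by pushing a zombie behavior tree asset onto it while active.
; On start it registers with the game mode, saves the original speed, boosts walk speed and applies poison-vent particles.
; While in use, a curve sets walk speed over time; ending pops the behavior, unregisters, restores speed and clears particles.
; The overlap handler is an empty stub.
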(event EventStartUse
  (params (Owner :type Actor%20Object%20Reference))
  (bind _returnvalue (Actor|GetComponentsByClass Owner "/Script/Engine.CharacterMovementComponent"))
  (bind _item (Utilities|Array|Get(acopy) _returnvalue))
  ;[1 1 1] Add power bt to controller
  (bind _returnvalue_2 (Class|JDBlueprintFunctionLibrary|PushBHTonNPC Owner "/Game/Powers/Effects/BHT/BHT_Power_Zombie.BHT_Power_Zombie"))
  (if _returnvalue_2
    (Class|BaseEffect|RegistertoGameMode)
    ;[1 1 1] Set Character Speed
    (Variables|Default|SetCharacterSpeed (Class|MovementComponent|GetMaxSpeed _item))
    (Variables|/Script/Engine.CharacterMovementComponent|SetMaxWalkSpeed _item 6e+02)
    ;[1 1 1] Set Particle Effect
    (Effects|Components|ParticleSystem|SetTemplate (Utilities|Array|Get(acopy) (Actor|GetComponentsByClass Owner "/Script/Engine.ParticleSystemComponent")) "/Game/Graphics/Vectorfields/Particles/P_PoisonVent.P_PoisonVent")
    ;[1 1 1] Bind On Overlap Event
    (Utilities|Casting|CastToBaseCharacter Owner)))

(event EventEndUse
  (params (Owner :type Actor%20Object%20Reference))
  ;[1 1 1] Remove power bht
  (bind _returnvalue (Class|JDBlueprintFunctionLibrary|PopBHTonNPC Owner))
  (if _returnvalue
    (Class|BaseEffect|UnregisterfromGameMode)
    ;[1 1 1] Remove Overlap Event
    (Utilities|Casting|CastToBaseCharacter Owner)
    ;[1 1 1] Remove Particle Effect
    (Variables|/Script/Engine.CharacterMovementComponent|SetMaxWalkSpeed (Utilities|Array|Get(acopy) (Actor|GetComponentsByClass Owner "/Script/Engine.CharacterMovementComponent")) (Variables|Default|GetCharacterSpeed))
    (Effects|Components|ParticleSystem|SetTemplate (Utilities|Array|Get(acopy) (Actor|GetComponentsByClass Owner "/Script/Engine.ParticleSystemComponent")) 0)
    (Variables|Default|SetTime 0.0)))

(event EventUsing
  (params (Owner :type Actor%20Object%20Reference) (DeltaTime :type Float%20%28single-precision%29))
  ;[1 1 1] Decrease Zombie Speed Over Time
  (bind _output_get (Variables|Default|SetTime (Variables|Default|GetTime)))
  (Variables|/Script/Engine.CharacterMovementComponent|SetMaxWalkSpeed (Utilities|Array|Get(acopy) (Actor|GetComponentsByClass Owner "/Script/Engine.CharacterMovementComponent")) (Math|Curves|GetFloatValue (Variables|Default|GetSpeedOverTime) _output_get)))

(fn BeginOverlap
  (params (Other%20Actor :type Actor%20Object%20Reference) (Other%20Comp :type Primitive%20Component%20Object%20Reference) (Other%20Body%20Index :type Integer) (From%20Sweep :type Boolean) (Sweep%20Result :type Boolean)))