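; BP_NPC is an NPC Blueprint that shows its current life on a world-space health counter widget.
; Each tick it copies the value from LifeComponent into the UI_HealtCounter widget hosted by the LifeCounter component.
; It then billboards the counter toward the player camera using only the look-at yaw with a fixed offset and roll, skipping both steps if the widget cast fails.
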(event EventTick
  (params (DeltaSeconds :type Float%20%28single-precision%29))
  (bind _lifecounter (Variables|Default|GetLifeCounter))
  ;[1 1 1] Set health counter value
  (bind _asui_healt_counter (Utilities|Casting|CastToUI_HealtCounter (UserInterface|GetUserWidgetObject (Variables|Default|GetLifeCounter))))
  (Variables|/Game/UI/Test/UI_HealtCounter.UI_HealtCounter_C|SetHealtValue _asui_healt_counter (Class|LifeComponent|GetLife (Variables|Default|GetLifeComponent)))
  ;[1 1 1] Rotate to face camera
  (Transformation|SetWorldRotation _lifecounter (Class|KismetMathLibrary|MakeRot 0.0 (- (.Yaw (Class|KismetMathLibrary|BreakRot (Math|Rotator|FindLookatRotation (Camera|GetCameraLocation (Game|GetPlayerCameraManager 0)) (Transformation|GetWorldLocation _lifecounter)))) -9e+01) 9e+01) false))

(fn ConstructionScript)