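; Game mode for free play that owns the level's UI and handles the end of a match.
; BeginPlay shows the free-mode widget.
; On WaitingPostMatch it swaps that for an end-game widget with result text, colored green or red by Won(), then quits the game after a short delay.
; EndPlay removes the end-game widget, noted as preventing a crash when opening the map.
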(event EventBeginPlay
  ;[1 1 1] Create and add the widget to the level
  (bind _returnvalue (UserInterface|CreateWidget "/Game/UI/UI_Free_GameMode.UI_Free_GameMode_C" (Game|GetPlayerController 0)))
  (Variables|Default|SetLevelMenuWidget _returnvalue)
  (UserInterface|Viewport|AddtoViewport _returnvalue 0))

(event EventOnSetMatchState
  (params (NewState :type Name))
  ;[1 1 1] Quit after match end and show match result widget
  (if (Utilities|Name|Equal(Name) NewState "WaitingPostMatch")
    (bind _returnvalue (UserInterface|CreateWidget "/Game/UI/UI_Game_End.UI_Game_End_C" (Game|GetPlayerController 0)))
    (bind _output_get (Variables|Default|SetEndGameWidget _returnvalue))
    ;;[1 1 1] Set the widget properties based on game result
    (bind _returnvalue_2 (Class|BaseBlankGameMode|GetEndGameDescription))
    (if (Class|BaseBlankGameMode|Won)
      (Variables|/Game/UI/UI_Game_End.UI_Game_End_C|SetMatchResultColor _output_get "(R=0.342857,G=0.800000,B=0.000000,A=1.000000)")
      (else
        (Variables|/Game/UI/UI_Game_End.UI_Game_End_C|SetMatchResultColor _output_get "(R=0.880000,G=0.000000,B=0.000000,A=1.000000)")))
    (Variables|/Game/UI/UI_Game_End.UI_Game_End_C|SetMatchResultText _output_get _returnvalue_2)
    (Widget|RemovefromParent (Variables|Default|GetLevelMenuWidget))
    (UserInterface|Viewport|AddtoViewport _output_get 0)
    (Utilities|FlowControl|Delay 5.0)
    (Game|QuitGame 0 "Quit")))

(event EventEndPlay
  (params (EndPlayReason :type EEndPlayReason%20Enum :default "ActorDestroyed"))
  ;[1 1 1] Clean the widget from the level, if this is not done opening the map will crash the game
  (Widget|RemovefromParent (Variables|Default|GetEndGameWidget)))

(fn ConstructionScript)