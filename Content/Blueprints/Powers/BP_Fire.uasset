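; BP_Fire is a fire power that spends souls to put a fire effect on a character.
; On Use, it spends souls first, then checks its box collider for overlapping BaseCharacter pawns.
; If any overlap, it creates a FireEffect object and adds it through the first character's EffectComponent.
; Souls are spent even when nothing overlaps.
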(event EventUse
  ;[1 1 1] Find the first actor overlapping the box component  and add an effect
  (Class|BasePowerActor|SpendSouls)
  (bind (_outactors _returnvalue) (Class|KismetSystemLibrary|ComponentOverlapActorsNEW (Variables|Default|GetBoxCollider) (Transformation|GetActorTransform) (Utilities|Array|MakeArray "ObjectTypeQuery3") "/Script/BaseBlank.BaseCharacter"))
  (if _returnvalue
    (bind _asbase_character (Utilities|Casting|CastToBaseCharacter (Utilities|Array|Get(acopy) _outactors)))
    (bind _returnvalue_2 (Class|JDBlueprintFunctionLibrary|CreateObject "/Game/Blueprints/Powers/Effects/FireEffect.FireEffect_C"))
    (bind _asbase_effect (Utilities|Casting|CastToBaseEffect _returnvalue_2))
    (Class|EffectComponent|AddEffect (Actor|GetComponentsByClass _asbase_character "/Script/BaseBlank.EffectComponent") _asbase_effect)))

(fn ConstructionScript)