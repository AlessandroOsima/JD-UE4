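; BP_Water is a placeable water surface actor for the stylized low-poly environment, built on the SMOceanWater mesh.
; The Construction Script calls MeshScale, which creates a dynamic instance of WaterMaterial on the mesh, stores it back in that variable, and sets horizontal scale from WaterScaleX and WaterScaleY.
; It then disables shadow casting on the mesh; the event graph holds no active logic.
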(event EventBeginPlay)

(event EventActorBeginOverlap
  (params (OtherActor :type Actor%20Object%20Reference)))

(event EventTick
  (params (DeltaSeconds :type Float%20%28single-precision%29)))

(fn ConstructionScript
  (CallFunction|MeshScale)
  (Rendering|SetCastShadow (Variables|Default|GetSM_OceanWater) false))

(fn MeshScale
  (bind _sm_oceanwater (Variables|Default|GetSM_OceanWater))
  (bind _returnvalue (Rendering|Material|CreateDynamicMaterialInstance _sm_oceanwater 0 (Variables|Default|GetWater%20Material) :!class /Script/Engine.PrimitiveComponent))
  (Variables|Default|SetWater%20Material _returnvalue)
  (Transformation|SetRelativeScale3D _sm_oceanwater (Math|Vector|MakeVector (Variables|Default|GetWater%20Scale%20X) (Variables|Default|GetWater%20Scale%20Y) 1.0)))